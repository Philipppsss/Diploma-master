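; Interactable bed with two sliding drawers that open and close through repeated interact calls, with door sounds.
; Each ActivateInteract calls the parent, then advances a four-state Open counter: open first drawer, open second, close second, close first.
; Two timelines lerp each drawer's relative location from its BeginPlay position toward an offset along Y, and reverse to close.
; The open_shelf events are leftover stubs that move nothing.
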(event `open_Shelf_2`
  (params (`open/close` :type Boolean))
  (if `open/close`
    _))

(event `self.Activate_interact`
  (params (Activate_Inteact :type Boolean))
  (bind _returnvalue (`self.K2_GetActorLocation`))
  (bind _returnvalue_2 (`self.K2_GetActorLocation`))
  (bind (_relativelocation_x _relativelocation_y _relativelocation_z) (`KismetMathLibrary.BreakVector` (`SceneComponent.RelativeLocation` (`self.SM_Bed_Drawer_Openable_Part_2`))))
  (bind (_relativelocation_x_2 _relativelocation_y_2 _relativelocation_z_2) (`KismetMathLibrary.BreakVector` (`SceneComponent.RelativeLocation` (`self.SM_Bed_Drawer_Openable_Part`))))
  (`parent.Activate_interact` Activate_Inteact)
  (switch `int` (`self.open`)
    (:`0`
      (set `self.open` 1)
      (`GameplayStatics.PlaySoundAtLocation` "/Game/Philipp/sounds/shelf_door_open.shelf_door_open" _returnvalue_2 (struct) 1.0 1.0 0.0 null null null)
      (set `self.end_loc` (`KismetMathLibrary.MakeVector` 0.0 (+ _relativelocation_y_2 100.0)))
      (bind (_direction _newtrack_0) (`Timeline|open_shelf_door` :!label _label)
        (:`Update`
          (`SceneComponent.K2_SetRelativeLocation` (`self.SM_Bed_Drawer_Openable_Part`) (`KismetMathLibrary.VLerp` (`self.start_loc`) (`self.end_loc`) _newtrack_0) false false))))
    (:`1`
      (set `self.open` 2)
      (`GameplayStatics.PlaySoundAtLocation` "/Game/Philipp/sounds/shelf_door_open.shelf_door_open" _returnvalue (struct) 1.0 1.0 0.0 null null null)
      (set `self.end_loc_2` (`KismetMathLibrary.MakeVector` _relativelocation_x (+ _relativelocation_y 100.0) _relativelocation_z))
      (bind (_direction_2 _newtrack_0_2) (`Timeline|Timeline_0` :!label _label_2)
        (:`Update`
          (`SceneComponent.K2_SetRelativeLocation` (`self.SM_Bed_Drawer_Openable_Part_2`) (`KismetMathLibrary.VLerp` (`self.start_loc_2`) (`self.end_loc_2`) _newtrack_0_2) false false))))
    (:`2`
      (set `self.open` 3)
      (`GameplayStatics.PlaySoundAtLocation` "/Game/Philipp/sounds/shelf_door_Close.shelf_door_Close" _returnvalue (struct) 1.0 1.0 0.0 null null null)
      (goto _label_2 :!via `Reverse`))
    (:`3`
      (set `self.open` 0)
      (`GameplayStatics.PlaySoundAtLocation` "/Game/Philipp/sounds/shelf_door_Close.shelf_door_Close" _returnvalue_2 (struct) 1.0 1.0 0.0 null null null)
      (goto _label :!via `Reverse`))))

(event `self.ReceiveBeginPlay`
  (bind (_relativelocation_x _relativelocation_y _relativelocation_z) (`KismetMathLibrary.BreakVector` (`SceneComponent.RelativeLocation` (`self.SM_Bed_Drawer_Openable_Part_2`))))
  (bind (_relativelocation_x_2 _relativelocation_y_2 _relativelocation_z_2) (`KismetMathLibrary.BreakVector` (`SceneComponent.RelativeLocation` (`self.SM_Bed_Drawer_Openable_Part`))))
  (`|ExecutionSequence`
    (:`then_0`
      (set `self.start_loc_2` (`KismetMathLibrary.MakeVector` _relativelocation_x _relativelocation_y _relativelocation_z)))
    (:`then_1`
      (set `self.start_loc` (`KismetMathLibrary.MakeVector` _relativelocation_x_2 _relativelocation_y_2 _relativelocation_z_2)))))

(event `open_shelf`
  (params (`open/close` :type Boolean))
  (set `self.open/close` `open/close`))

(fn `UserConstructionScript`)